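; Bomb bot AI character that wanders to random reachable points, chases the player on sight and self-destructs when it reaches them.
; An armed bot explodes after a short delay, damaging the player if the BlastRadious overlap flag is set.
; Hammer overlaps reduce health according to the player's attack type, with only default-attack kills granting energy and possible TimeFragment drops.
; Both death paths decrement the game mode's bot count.
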(event `self.ReceiveActorBeginOverlap`
  (params (OtherActor :type "Actor Object Reference"))
  ;[1 1 1] damage system
)

(event `self.CapsuleComponent.OnComponentBeginOverlap`
  (params (OverlappedComponent :type "PrimitiveComponent Object Reference") (OtherActor :type "Actor Object Reference") (OtherComp :type "PrimitiveComponent Object Reference") (OtherBodyIndex :type Integer) (bFromSweep :type Boolean) (SweepResult :type "HitResult Structure (by ref)"))
  ;[1 1 1] damage system
  (cast `/Game/BOT/Blueprints/Hammer` OtherActor)
  (bind _asthird_person_character (cast `/Game/BOT/Blueprints/ThirdPersonCharacter` (`GameplayStatics.GetPlayerCharacter` 0)))
  (switch `int` (`/Game/BOT/Blueprints/ThirdPersonCharacter.DamageType` _asthird_person_character)
    (:`1`
      ;;[1 1 1] default attack
      (set `self.Health` (- (`self.Health`) 0.5))
      (if (<= (`self.Health`) 0.0)
        (`GameplayStatics.SpawnEmitterAtLocation` "/Game/StarterContent/Particles/P_Explosion.P_Explosion" (`SceneComponent.K2_GetComponentLocation` (`self.Mesh`)))
        (bind _attackenergy (`/Game/BOT/Blueprints/ThirdPersonCharacter.AttackEnergy` _asthird_person_character))
        (if (< _attackenergy 12.0)
          (`/Engine/EditorBlueprintResources/StandardMacros.IncrementFloat` _attackenergy
            (:`  `
              _)))
        (if (> (`KismetMathLibrary.RandomIntegerInRange` 0 3) 0)
          (`|SpawnActorFromClass` "/Game/BOT/Blueprints/TimeFragment.TimeFragment_C" (`SceneComponent.K2_GetComponentToWorld` (`self.Mesh`)) "Undefined" "OverrideRootScale" null null))
        (bind _asthird_person_game_mode (cast `/Game/BOT/Blueprints/ThirdPersonGameMode` (`GameplayStatics.GetGameMode`) :!label _label))
        (`/Engine/EditorBlueprintResources/StandardMacros.DecrementInt` (`/Game/BOT/Blueprints/ThirdPersonGameMode.number of bots` _asthird_person_game_mode)
          (:`  `
            (`KismetSystemLibrary.PrintString` "bomb destroyed")
            (`self.K2_DestroyActor`)))))
    (:`2`
      ;;[1 1 1] helicopter
      (set `self.Health` (- (`self.Health`) 0.4))
      (if (<= (`self.Health`) 0.0) :!label _label_2
        (`GameplayStatics.SpawnEmitterAtLocation` "/Game/StarterContent/Particles/P_Explosion.P_Explosion" (`SceneComponent.K2_GetComponentLocation` (`self.Mesh`)))
        (goto _label)))
    (:`3`
      ;;[1 1 1] hand helicopter
      (set `self.Health` (- (`self.Health`) 0.5))
      (goto _label_2))
    (:`4`
      ;;[1 1 1] jump splash
      (set `self.Health` (- (`self.Health`) 1.0))
      (goto _label_2))))

(event `self.ReceiveBeginPlay`
  ;[1 1 1] move to random location
  (if (not (`self.AI_moving?`)) :!label _label_3
    (set `self.AI_moving?` true)
    (`|AIMoveTo` self (`NavigationSystemV1.K2_GetRandomReachablePointInRadius` (`self.K2_GetActorLocation`) 5000.0 null null) null
      (:`then`
        _)
      (:`OnSuccess`
        (set `self.AI_moving?` false :!label _label_4))
      (:`OnFail`
        (goto _label_4)))
    (`KismetSystemLibrary.Delay` 2.0)
    (goto _label_3)))

(event `self.PawnSensing.OnSeePawn`
  (params (Pawn :type "Pawn Object Reference"))
  (bind _returnvalue (`SceneComponent.K2_GetComponentLocation` (`self.Mesh`)))
  (`KismetSystemLibrary.PrintString` (`KismetSystemLibrary.GetDisplayName` Pawn))
  (bind _asthird_person_character (cast `/Game/BOT/Blueprints/ThirdPersonCharacter` (`GameplayStatics.GetPlayerCharacter` 0)))
  (set `self.AI_moving?` true)
  ;[1 1 1] chase player
  (`|AIMoveTo` self (0.0 0.0 0.0) _asthird_person_character
    (:`then`
      (set `self.AI_moving?` false))
    (:`OnSuccess`
      ;[1 1 1] explod on player
      (set `self.Armed` true)
      (`KismetSystemLibrary.Delay` 2.0)
      (`GameplayStatics.SpawnEmitterAtLocation` "/Game/StarterContent/Particles/P_Explosion.P_Explosion" _returnvalue (struct) (3.0 3.0 3.0))
      (`GameplayStatics.PlaySoundAtLocation` "/Game/StarterContent/Audio/Explosion_Cue.Explosion_Cue" _returnvalue (struct) 1.0 1.0 0.0 null null null)
      (if (`self.player in radious`)
        (set `/Game/BOT/Blueprints/ThirdPersonCharacter.Health` (- (`/Game/BOT/Blueprints/ThirdPersonCharacter.Health` _asthird_person_character) (`self.blastdamage`)) _asthird_person_character))
      (set `self.AI_moving?` false)
      (bind _asthird_person_game_mode (cast `/Game/BOT/Blueprints/ThirdPersonGameMode` (`GameplayStatics.GetGameMode`)))
      (`/Engine/EditorBlueprintResources/StandardMacros.DecrementInt` (`/Game/BOT/Blueprints/ThirdPersonGameMode.number of bots` _asthird_person_game_mode)
        (:`  `
          (`KismetSystemLibrary.PrintString` "bomb blast")
          (`self.K2_DestroyActor`))))
    (:`OnFail`
      (set `self.AI_moving?` false))))

(event `self.blast radious.OnComponentBeginOverlap`
  (params (OverlappedComponent :type "PrimitiveComponent Object Reference") (OtherActor :type "Actor Object Reference") (OtherComp :type "PrimitiveComponent Object Reference") (OtherBodyIndex :type Integer) (bFromSweep :type Boolean) (SweepResult :type "HitResult Structure (by ref)"))
  ;[1 1 1] set player in blast radious
  (set `self.player in radious` true)
  (cast `/Game/BOT/Blueprints/ThirdPersonCharacter` OtherActor))

(event `self.blast radious.OnComponentEndOverlap`
  (params (OverlappedComponent :type "PrimitiveComponent Object Reference") (OtherActor :type "Actor Object Reference") (OtherComp :type "PrimitiveComponent Object Reference") (OtherBodyIndex :type Integer))
  ;[1 1 1] set player in blast radious
  (set `self.player in radious` false)
  (cast `/Game/BOT/Blueprints/ThirdPersonCharacter` OtherActor))

(fn `UserConstructionScript`
  (`parent.UserConstructionScript`))