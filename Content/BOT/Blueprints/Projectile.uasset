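; Projectile actor in the BOT folder that damages a ThirdPersonCharacter on contact and destroys itself after a fixed lifetime.
; When its static mesh overlaps that character, it subtracts directly from the Health variable and spawns a scaled-down explosion emitter at its location.
; After a brief delay it destroys the emitter and itself; overlaps with other actor types are ignored.
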(event `self.ReceiveBeginPlay`
  (`KismetSystemLibrary.Delay` 5.0)
  (`self.K2_DestroyActor`))

(event `self.projectile_StaticMesh.OnComponentBeginOverlap`
  (params (OverlappedComponent :type "PrimitiveComponent Object Reference") (OtherActor :type "Actor Object Reference") (OtherComp :type "PrimitiveComponent Object Reference") (OtherBodyIndex :type Integer) (bFromSweep :type Boolean) (SweepResult :type "HitResult Structure (by ref)"))
  (bind _asthird_person_character (cast `/Game/BOT/Blueprints/ThirdPersonCharacter` OtherActor))
  (set `/Game/BOT/Blueprints/ThirdPersonCharacter.Health` (- (`/Game/BOT/Blueprints/ThirdPersonCharacter.Health` _asthird_person_character) 5) _asthird_person_character)
  (bind _returnvalue (`GameplayStatics.SpawnEmitterAtLocation` "/Game/StarterContent/Particles/P_Explosion.P_Explosion" (`self.K2_GetActorLocation`) (struct) (0.5 0.5 0.5) false))
  (`KismetSystemLibrary.Delay` 0.1)
  (`ActorComponent.K2_DestroyComponent` _returnvalue)
  (`self.K2_DestroyActor`))

(fn `UserConstructionScript`)