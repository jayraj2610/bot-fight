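; Health pickup actor that restores a fixed amount of health to an overlapping ThirdPersonCharacter.
; It only applies when the character is below its current max health, adding health without clamping, printing the new value and playing a powerup sound before destroying itself.
; Uncollected fragments destroy themselves after a timed delay from BeginPlay, sharing the same destroy node.
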(event `self.ReceiveBeginPlay`
  (`KismetSystemLibrary.Delay` 30.0)
  (`self.K2_DestroyActor` :!label _label))

(event `self.ReceiveActorBeginOverlap`
  (params (OtherActor :type "Actor Object Reference"))
  (bind _asthird_person_character (cast `/Game/BOT/Blueprints/ThirdPersonCharacter` OtherActor))
  (bind _health (`/Game/BOT/Blueprints/ThirdPersonCharacter.Health` _asthird_person_character))
  (if (< _health (`/Game/BOT/Blueprints/ThirdPersonCharacter.currentmax_health` _asthird_person_character))
    (bind _output_get (set `/Game/BOT/Blueprints/ThirdPersonCharacter.Health` (+ _health 30) _asthird_person_character))
    (`KismetSystemLibrary.PrintString` (`KismetStringLibrary.Conv_IntToString` _output_get))
    (`GameplayStatics.PlaySoundAtLocation` "/Game/sound/Special_Powerup_01_wav.Special_Powerup_01_wav" (`self.K2_GetActorLocation`) (struct) 1.0 1.0 0.0 null null null)
    (goto _label)))

(fn `UserConstructionScript`)