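; Spawner Blueprint that places AI bots at random reachable navigation points around its own location.
; SpawnExplosivebot spawns a bomb bot within a wide radius, while Spawnturretbot uses a smaller radius and keeps the spawner's height.
; Each function then increments NumberOfBots on ThirdPersonGameMode.
; Its event graph is empty, so spawning depends on calls from outside.
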(fn `spawnExplosivebot`
  (`AIBlueprintHelperLibrary.SpawnAIFromClass` "/Game/BOT/Blueprints/BOMB_Bot_ai_character.BOMB_Bot_ai_character_C" null (`NavigationSystemV1.K2_GetRandomReachablePointInRadius` (`self.K2_GetActorLocation`) 7000.0 null null) (struct) false null)
  (bind _asthird_person_game_mode (cast `/Game/BOT/Blueprints/ThirdPersonGameMode` (`GameplayStatics.GetGameMode`)))
  (`/Engine/EditorBlueprintResources/StandardMacros.IncrementInt` (`/Game/BOT/Blueprints/ThirdPersonGameMode.number of bots` _asthird_person_game_mode)))

(fn `spawnturretbot`
  (locals (NewLocalVar_0 :type "Vector Structure" :default (0.0 0.0 0.0)))
  (bind (_returnvalue_x _returnvalue_y _returnvalue_z) (`KismetMathLibrary.BreakVector` (`self.K2_GetActorLocation`)))
  (bind _randomlocation (`NavigationSystemV1.K2_GetRandomReachablePointInRadius` (`KismetMathLibrary.MakeVector` _returnvalue_x _returnvalue_y _returnvalue_z) 5000.0 null null))
  (`AIBlueprintHelperLibrary.SpawnAIFromClass` "/Game/BOT/Blueprints/TURRENT_bot_ai_chracter.TURRENT_bot_ai_chracter_C" null (`KismetMathLibrary.MakeVector` (.x _randomlocation) (.y _randomlocation) _returnvalue_z) (struct) false null)
  (bind _asthird_person_game_mode (cast `/Game/BOT/Blueprints/ThirdPersonGameMode` (`GameplayStatics.GetGameMode`)))
  (`/Engine/EditorBlueprintResources/StandardMacros.IncrementInt` (`/Game/BOT/Blueprints/ThirdPersonGameMode.number of bots` _asthird_person_game_mode)))

(fn `UserConstructionScript`)