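; BotAI_character is a bot character Blueprint that takes damage from the player's hammer.
; On overlap with a Hammer actor, it checks whether player zero's ThirdPersonCharacter is attacking.
; If so, it prints a debug hit message, subtracts a fixed amount from Health, and destroys itself once Health reaches zero or below.
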(event `self.ReceiveActorBeginOverlap`
  (params (OtherActor :type "Actor Object Reference"))
  (cast `/Game/BOT/Blueprints/Hammer` OtherActor)
  (bind _asthird_person_character (cast `/Game/BOT/Blueprints/ThirdPersonCharacter` (`GameplayStatics.GetPlayerCharacter` 0)))
  (if (`/Game/BOT/Blueprints/ThirdPersonCharacter.isAttacking` _asthird_person_character)
    (`KismetSystemLibrary.PrintString` "hit")
    (bind _output_get (set `self.Health` (- (`self.Health`) 0.4)))
    (if (<= _output_get 0.0)
      (`self.K2_DestroyActor`))))

(fn `UserConstructionScript`)