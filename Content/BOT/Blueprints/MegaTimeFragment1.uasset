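; MegaTimeFragment1 is a timed pickup actor that awards a large batch of time fragments to the player.
; When the player character overlaps it, it adds a fixed amount to the ThirdPersonCharacter's TimeFragments and destroys itself.
; An uncollected fragment also destroys itself after a delay that starts on BeginPlay.
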(event `self.ReceiveBeginPlay`
  (`KismetSystemLibrary.Delay` 30.0)
  (`self.K2_DestroyActor` :!label _label))

(event `self.ReceiveActorBeginOverlap`
  (params (OtherActor :type "Actor Object Reference"))
  (if (== OtherActor (`GameplayStatics.GetPlayerCharacter` 0))
    (bind _asthird_person_character (cast `/Game/BOT/Blueprints/ThirdPersonCharacter` (`GameplayStatics.GetPlayerCharacter` 0)))
    (set `/Game/BOT/Blueprints/ThirdPersonCharacter.TimeFragments` (+ (`/Game/BOT/Blueprints/ThirdPersonCharacter.TimeFragments` _asthird_person_character) 150) _asthird_person_character)
    (goto _label)))

(fn `UserConstructionScript`)